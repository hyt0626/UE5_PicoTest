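; TrackerData is a Blueprint that reads pass-through data from PICO XR external tracker devices to detect a fire key press.
; BeginPlay enables the pass-through state on Android only and stores the result in IsEnablePass.
; While that flag is set, Tick polls every data packet and treats byte 4 equal to 1 as fire.
; The only response is a debug PrintString, shown on screen when pressed.
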(event EventBeginPlay
  (if (Utilities|Enum|Equal(Enum) (Game|GetPlatformName) "Android")
    (bind _returnvalue (Class|PICOXRMotionTrackingFunctionLibrary|PXRSetExtDevTrackerPassDataState true))
    (Variables|Default|SetisEnablePass _returnvalue)))

(event EventTick
  (params (DeltaSeconds :type Float%20%28single-precision%29))
  (if (Variables|Default|GetisEnablePass)
    (bind _passdatas (Class|PICOXRMotionTrackingFunctionLibrary|PXRGetExtDevTrackerbyPassData))
    (for _array_element _passdatas
      (Development|PrintString "啪" (== (Utilities|Array|Get(acopy) (.PassData (Utilities|Struct|BreakPXRExtDevTrackerPassData _array_element)) 4) 1)))))