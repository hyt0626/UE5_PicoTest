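; TCP client Blueprint that registers with a server as "VR2" using hardcoded details and exchanges typed JSON command messages.
; Tick calls Connect whenever disconnected; connecting triggers registration, and Space sends a hardcoded test command.
; Outgoing structs become JSON packets.
; Received bytes accumulate in a buffer, drained by a capped packet-popping loop; only command responses (type 13) are deserialized and printed.
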(event OnReceivedBytes(TCPClient)
  (params (Bytes :type Array%20of%20Bytes))
  (CallFunction|RecvFeed Bytes))

(event OnConnected(TCPClient)
  (Variables|Default|SetbConnected true)
  (CallFunction|SendRegister))

(event OnDisconnected(TCPClient)
  (Variables|Default|SetbConnected false))

(event EventBeginPlay)

(event Collision|EventActorBeginOverlap
  (params (OtherActor :type Actor%20Object%20Reference)))

(event EventTick
  (params (DeltaSeconds :type Float%20%28single-precision%29))
  (if (not (Variables|Default|GetbConnected))
    (CallFunction|Connect)))

(event EventEndPlay
  (params (EndPlayReason :type EEndPlayReason%20Enum :default "Destroyed")))

(event Input|KeyboardEvents|SpaceBar
  (params (Key :type Key%20Structure :default "None"))
  (:Pressed
    (CallFunction|SendCom)))

(fn ConstructionScript)

(fn BPSendMessage
  (params (Type :type Integer) (JsonString :type String))
  (Class|TCPClientComponent|Emit (Variables|Default|GetTCPClient) (Class|TcpPacketBP|BuildPacketfromJson Type JsonString)))

(fn BPRecvFeed
  (params (InBytes :type Array%20of%20Bytes))
  (bind _recvbuffer (Variables|Default|GetRecvBuffer))
  (Utilities|Array|AppendArray _recvbuffer InBytes)
  (Utilities|FlowControl|ForLoopwithBreak 0 50 :!label _label
    (:LoopBody
      (bind (_outtype _outjsonstring _returnvalue) (Class|TcpPacketBP|TryPopPacket _recvbuffer))
      (if _returnvalue
        (CallFunction|ParsetoStruct _outtype _outjsonstring)
        (else
          (goto _label Break))))))

(fn BPSendRegister
  (bind _outjsonstring (|StructtoJsonString (Utilities|Struct|MakeST_Register 2 "VR2" "12345678901234567")))
  (CallFunction|SendMessage 1 _outjsonstring))

(fn BPSendCom
  (bind _outjsonstring (|StructtoJsonString (Utilities|Struct|MakeST_Com "12345678901234567" "小明" 0 1 "打击")))
  (CallFunction|SendMessage 13 _outjsonstring))

(fn BPParsetoStruct
  (params (Type :type Integer) (Json :type String))
  (switch int Type
    (:13
      (bind _outstruct (Class|EasyJsonUtils|EasyDeserialize Json))
      (bind _output_get (Variables|Default|SetST_ComResp _outstruct))
      (CallFunction|HandleComResp _output_get))))

(fn BPHandleComResp
  (params (Com :type ST%20Com%20Structure))
  (Development|PrintString (.str Com)))

(fn BPConnect
  (bind _st_tcpaddress (Variables|Default|GetST_TcpAddress))
  (Class|TCPClientComponent|ConnecttoSocketasClient (Variables|Default|GetTCPClient) (.ip _st_tcpaddress) (.port _st_tcpaddress)))