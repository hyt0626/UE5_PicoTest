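; TCP client actor that links a VR station to a fixed-address server, apparently as a test harness with hardcoded identity and payloads.
; It connects on BeginPlay, retries through a delayed Tick while disconnected, and sends registration plus a sample command once connected.
; Outgoing structs become JSON wrapped in typed packets.
; Incoming bytes accumulate in a buffer, are drained in a bounded packet loop, and command responses are deserialized and printed.
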(event Custom|TCP_OnDisConnected
  (params (ConnectionId :type Integer))
  (Variables|Default|SetbConnected false))

(event Custom|TCP_OnConnected
  (params (ConnectionId :type Integer))
  (Variables|Default|SetbConnected true)
  (CallFunction|SendRegister)
  (CallFunction|SendCom))

(event Custom|TCP_OnMessageReceived
  (params (ConnectionId :type Integer) (Message :type Array%20of%20Bytes))
  (CallFunction|RecvFeed Message))

(event EventBeginPlay
  (CallFunction|Connect))

(event Collision|EventActorBeginOverlap
  (params (OtherActor :type Actor%20Object%20Reference)))

(event EventTick
  (params (DeltaSeconds :type Float%20%28single-precision%29))
  (if (not (Variables|Default|GetbConnected))
    (Utilities|FlowControl|Delay 3.0)
    (CallFunction|Connect)))

(fn ConstructionScript)

(fn BPConnect
  (bind _connectionid (Class|TcpSocketConnection|Connect "192.168.66.100" 3000 (EventDispatchers|CreateEvent :!event Custom|TCP_OnDisConnected) (EventDispatchers|CreateEvent :!event Custom|TCP_OnConnected) (EventDispatchers|CreateEvent :!event Custom|TCP_OnMessageReceived)))
  (Variables|Default|SetConnection%20Id _connectionid))

(fn BPSendRegister
  (bind _outjsonstring (|StructtoJsonString (Utilities|Struct|MakeST_Register 2 "VR2" "12345678901234567")))
  (CallFunction|SendMessage 1 _outjsonstring))

(fn BPRecvFeed
  (params (InBytes :type Array%20of%20Bytes))
  (bind _recvbuffer (Variables|Default|GetRecvBuffer))
  (Utilities|Array|AppendArray _recvbuffer InBytes)
  (Utilities|FlowControl|ForLoopwithBreak 0 50 :!label _label
    (:LoopBody
      (bind (_outtype _outjsonstring _returnvalue) (Class|TcpPacketBP|TryPopPacket _recvbuffer))
      (if _returnvalue
        (CallFunction|ParsetoStruct _outtype _outjsonstring)
        (else
          (goto _label Break))))))

(fn BPSendMessage
  (params (Type :type Integer) (JsonString :type String))
  (Class|TcpSocketConnection|SendData (Variables|Default|GetConnection%20Id) (Class|TcpPacketBP|BuildPacketfromJson Type JsonString)))

(fn BPParsetoStruct
  (params (Type :type Integer) (Json :type String))
  (switch int Type
    (:13
      (bind _outstruct (Class|EasyJsonUtils|EasyDeserialize Json))
      (bind _output_get (Variables|Default|SetST_ComResp _outstruct))
      (CallFunction|HandleComResp _output_get))))

(fn BPHandleComResp
  (params (Com :type ST%20Com%20Structure))
  (bind _outjsonstring (|StructtoJsonString Com))
  (Development|PrintString _outjsonstring))

(fn BPSendCom
  (bind _outjsonstring (|StructtoJsonString (Utilities|Struct|MakeST_Com "12345678901234567" "小明" 0 1 "打击A玩家")))
  (CallFunction|SendMessage 13 _outjsonstring))